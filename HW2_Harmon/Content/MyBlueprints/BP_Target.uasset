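; BP_Target is a shootable target that counts toward the player's goal when destroyed.
; Each hit from a BP_FirstPersonProjectile removes a fixed amount of Health, and other hits are ignored.
; When Health runs out, it increments TargetsHit on the player's BP_FirstPersonCharacter, calls CheckGoal there, then destroys itself.
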(event Collision|EventHit
  (params (MyComp :type Primitive%20Component%20Object%20Reference) (Other :type Actor%20Object%20Reference) (OtherComp :type Primitive%20Component%20Object%20Reference) (bSelfMoved :type Boolean) (HitLocation :type Vector :default "0, 0, 0") (HitNormal :type Vector :default "0, 0, 0") (NormalImpulse :type Vector :default "0, 0, 0") (Hit :type Hit%20Result%20Structure%20%28by%20ref%29))
  (Utilities|Casting|CastToBP_FirstPersonProjectile Other)
  (Variables|Default|SetHealth (- (Variables|Default|GetHealth) 50))
  (if (<= (Variables|Default|GetHealth) 0)
    (bind _asbp_first_person_character (Utilities|Casting|CastToBP_FirstPersonCharacter (Game|GetPlayerCharacter 0)))
    (Math|Integer|IncrementInt (Variables|/Game/FirstPerson/Blueprints/BP_FirstPersonCharacter.BP_FirstPersonCharacter_C|GetTargetsHit _asbp_first_person_character)
      (:%20%20
        (Default|CheckGoal _asbp_first_person_character)
        (Actor|DestroyActor)))))

(fn ConstructionScript)